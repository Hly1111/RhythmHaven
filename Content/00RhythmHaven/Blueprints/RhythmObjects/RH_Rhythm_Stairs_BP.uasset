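; RH_Rhythm_Stairs_BP is a rhythm-driven stair object that animates its vertical scale on each beat event.
; On each beat it sets a timeline play rate from the inverse of TweenTime, captures the root's current Z scale and plays TL_Stair from the start.
; Timeline updates multiply that captured scale by the curve value, leaving X and Y unchanged.
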(event OnBeatEvent(Rhythm)
  (params (Bar :type Integer) (Beat :type Integer))
  (bind _root (Variables|Default|GetRoot))
  (bind _relativescale3d (Variables|/Script/Engine.SceneComponent|GetRelativeScale3D _root))
  (Components|Timeline|SetPlayRate (Variables|Default|GetTL_Stair) (/ 1.0 (Variables|Default|GetTweenTime)))
  (Variables|Default|SetStartZ (.z (Variables|/Script/Engine.SceneComponent|GetRelativeScale3D (Variables|Default|GetRoot))))
  (bind _t (Timeline|TL_Stair PlayFromStart)
    (:Update
      (Transformation|SetRelativeScale3D _root (Math|Vector|MakeVector (.x _relativescale3d) (.y _relativescale3d) (* _t (Variables|Default|GetStartZ)))))))

(event EventBeginPlay)

(event Collision|EventActorBeginOverlap
  (params (OtherActor :type Actor%20Object%20Reference)))

(event EventTick
  (params (DeltaSeconds :type Float%20%28single-precision%29)))

(fn ConstructionScript)