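; Rhythm sign actor that slides vertically in time with the beat.
; The Rhythm beat event alternates the TL_Sign timeline forward and backward on even and odd beats, with Reverse flipping the phase.
; TweenTime sets the play rate, and the timeline output drives the Root's relative Z up to a scale of 400 units while keeping X and Y.
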(event OnBeatEvent(Rhythm)
  (params (Bar :type Integer) (Beat :type Integer))
  (bind _root (Variables|Default|GetRoot))
  (bind _relativelocation (Variables|/Script/Engine.SceneComponent|GetRelativeLocation _root))
  (Components|Timeline|SetPlayRate (Variables|Default|GetTL_Sign) (/ 1.0 (Variables|Default|GetTweenTime)))
  (if (== (Math|Integer|%(Integer) Beat 2) 0)
    (if (Variables|Default|GetbReverse)
      (bind _t (Timeline|TL_Sign Reverse)
        (:Update
          (Transformation|SetRelativeLocation _root (Math|Vector|MakeVector (.x _relativelocation) (.y _relativelocation) (* _t 4e+02)) false false)))
      (else
        (Timeline|TL_Sign Play)))
    (elif (Variables|Default|GetbReverse)
      (Timeline|TL_Sign Play)
      (else
        (Timeline|TL_Sign Reverse)))))

(event EventBeginPlay)

(event Collision|EventActorBeginOverlap
  (params (OtherActor :type Actor%20Object%20Reference)))

(event EventTick
  (params (DeltaSeconds :type Float%20%28single-precision%29)))

(fn ConstructionScript)