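; RH_Rhythm_Platform is a rhythm object: a platform that moves up and down in time with the beat.
; Each Rhythm OnBeatEvent flips a FlipFlop that alternately plays and reverses a timeline, offsetting the root's relative Z by up to the curve value times a fixed 800 units, with sweep.
; BeginPlay caches the starting height and derives the timeline play rate from TweenTime.
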(event OnBeatEvent(Rhythm)
  (params (Bar :type Integer) (Beat :type Integer))
  (bind _root (Variables|Default|GetRoot))
  (bind _relativelocation (Variables|/Script/Engine.SceneComponent|GetRelativeLocation _root))
  (Utilities|FlowControl|Sequence
    (:then_1
      (Utilities|FlowControl|FlipFlop
        (:A
          (bind _t (Timeline|TL_Platform Play)
            (:Update
              (Transformation|SetRelativeLocation _root (Math|Vector|MakeVector (.x _relativelocation) (.y _relativelocation) (+ (* _t 8e+02) (Variables|Default|GetStartZ))) true false))))
        (:B
          (Timeline|TL_Platform Reverse))))))

(event EventBeginPlay
  (|CallParentFunction)
  (Components|Timeline|SetPlayRate (Variables|Default|GetTL_Platform) (/ 1.0 (Variables|Default|GetTweenTime)))
  (Variables|Default|SetStartZ (.z (Variables|/Script/Engine.SceneComponent|GetRelativeLocation (Variables|Default|GetRoot)))))

(event Collision|EventActorBeginOverlap
  (params (OtherActor :type Actor%20Object%20Reference)))

(event EventTick
  (params (DeltaSeconds :type Float%20%28single-precision%29)))

(fn ConstructionScript)