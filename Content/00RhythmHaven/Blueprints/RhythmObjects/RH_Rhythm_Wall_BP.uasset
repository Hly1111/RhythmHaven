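; RH_Rhythm_Wall_BP is a rhythm wall that moves and rotates its Hinge in response to Rhythm beat events.
; Beat 1 plays a fast timeline that slides the hinge along world X from its current position.
; Beats 3 and 4 call StartDoorTween to swing the hinge halfway, then fully, toward its closed yaw.
; Each tween starts from the current alpha, with timeline play rate derived from TweenTime.
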(event OnBeatEvent(Rhythm)
  (params (Bar :type Integer) (Beat :type Integer))
  (bind _hinge (Variables|Default|GetHinge))
  (bind _returnvalue (Transformation|GetWorldLocation _hinge))
  (switch int Beat
    (:1
      (Components|Timeline|SetPlayRate (Variables|Default|GetTimeline) 5.0)
      (Variables|Default|SetStartX (.x (Transformation|GetWorldLocation (Variables|Default|GetHinge))))
      (bind _t (Timeline|Timeline Play)
        (:Update
          (Transformation|SetWorldLocation (Variables|Default|GetHinge) (Math|Vector|MakeVector (+ (Variables|Default|GetStartX) (* _t 4e+02)) (.y _returnvalue) (.z _returnvalue)) false false))))
    (:3
      (CallFunction|StartDoorTween 0.5))
    (:4
      (CallFunction|StartDoorTween 1.0))))

(event Custom|StartDoorTween
  (params (Target :type Float%20%28double-precision%29))
  (Variables|Default|SetStartAlpha (Variables|Default|GetCurrentAlpha))
  (Variables|Default|SetTargetAlpha Target)
  (Components|Timeline|SetPlayRate (Variables|Default|GetTL_Door) (/ 1.0 (Variables|Default|GetTweenTime)))
  (bind _t (Timeline|TL_Door PlayFromStart)
    (:Update
      (bind _output_get (Variables|Default|SetCurrentAlpha (Math|Float|Lerp (Variables|Default|GetStartAlpha) (Variables|Default|GetTargetAlpha) _t)))
      (Transformation|SetRelativeRotation (Variables|Default|GetHinge) (Math|Rotator|MakeRotator 0.0 0.0 (Math|Float|Lerp (Variables|Default|GetOpenYaw) (Variables|Default|GetClosedYaw) _output_get)) false false))))

(event EventBeginPlay)

(event Collision|EventActorBeginOverlap
  (params (OtherActor :type Actor%20Object%20Reference)))

(event EventTick
  (params (DeltaSeconds :type Float%20%28single-precision%29)))

(fn ConstructionScript)