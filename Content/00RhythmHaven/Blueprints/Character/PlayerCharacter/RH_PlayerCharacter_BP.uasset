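; Player character Blueprint that deals melee damage to enemies through a weapon hitbox.
; When WeaponBox overlaps an actor tagged Enemy, it sends that actor a damage message with the box's hit parameters and itself as instigator.
; A DamagedActors list limits each enemy to one hit until the hitbox disarms and clears it.
; Incoming EnemyReceiveDamage events pass straight to the parent implementation.
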(event OnComponentBeginOverlap(WeaponBox)
  (params (OverlappedComponent :type Primitive%20Component%20Object%20Reference) (OtherActor :type Actor%20Object%20Reference) (OtherComp :type Primitive%20Component%20Object%20Reference) (OtherBodyIndex :type Integer) (bFromSweep :type Boolean) (SweepResult :type Hit%20Result%20Structure%20%28by%20ref%29))
  (bind _damagedactors (Variables|Default|GetDamagedActors))
  (if (Actor|ActorHasTag OtherActor "Enemy")
    (if (not (Utilities|Array|IsValidIndex _damagedactors (Utilities|Array|FindItem _damagedactors OtherActor)))
      (Utilities|Array|AddUnique (Variables|Default|GetDamagedActors) OtherActor)
      (Class|RHCharacterActionInterface|EnemyReceiveDamage(Message) OtherActor (Class|WeaponHitBox|GetParams (Variables|Default|GetWeaponBox)) self))))

(event OnDisarmHitBox(WeaponBox)
  (Utilities|Array|Clear (Variables|Default|GetDamagedActors)))

(event EventBeginPlay)

(event Collision|EventActorBeginOverlap
  (params (OtherActor :type Actor%20Object%20Reference)))

(event EventTick
  (params (DeltaSeconds :type Float%20%28single-precision%29)))

(event EventEnemyReceiveDamage
  (params (HitData :type RH%20Hit%20Params%20Structure) (AttackInstigator :type Character%20Object%20Reference))
  (|CallParentFunction HitData AttackInstigator))

(fn ConstructionScript)