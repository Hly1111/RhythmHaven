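; Enemy character Blueprint for Rhythm Haven that attacks the player and dies in an explosion when its health runs out.
; Attacks activate GAS abilities by the Attack.EnemyAttack tag.
; The weapon hitbox sends its hit data to Player-tagged actors, limited to one hit until the hitbox disarms.
; AttributeSet health changes update the health bar widget, or spawn the explosion and destroy the actor at zero.
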(event OnDisarmHitBox(WeaponHitBox)
  (Variables|Default|SetbHasHitPlayer false))

(event OnComponentBeginOverlap(WeaponHitBox)
  (params (OverlappedComponent :type Primitive%20Component%20Object%20Reference) (OtherActor :type Actor%20Object%20Reference) (OtherComp :type Primitive%20Component%20Object%20Reference) (OtherBodyIndex :type Integer) (bFromSweep :type Boolean) (SweepResult :type Hit%20Result%20Structure%20%28by%20ref%29))
  (if (Actor|ActorHasTag OtherActor "Player")
    (if (not (Variables|Default|GetbHasHitPlayer))
      (Variables|Default|SetbHasHitPlayer true)
      (Class|RHCharacterActionInterface|EnemyReceiveDamage(Message) OtherActor (Class|WeaponHitBox|GetParams (Variables|Default|GetWeaponHitBox)) self))))

(event OnHealthChanged(AttributeSet)
  (params (NewHealth :type Float%20%28single-precision%29) (MaxHealth :type Float%20%28single-precision%29))
  (if (<= NewHealth 0.0)
    (Niagara|SpawnSystematLocation "/Game/VFX_PackVol2/Effects/P_Explosion_01_Converted.P_Explosion_01_Converted" (Transformation|GetActorLocation) "0, 0, 0" "0.500000,0.500000,0.500000" true true "AutoRelease")
    (Actor|DestroyActor)
    (else
      (bind _asrh_enemy_stats_wb (Utilities|Casting|CastToRH_EnemyStats_WB (UserInterface|GetWidget (Variables|Default|GetHealthBar))))
      (Default|SetHealth _asrh_enemy_stats_wb NewHealth MaxHealth))))

(event EventBeginPlay)

(event Collision|EventActorBeginOverlap
  (params (OtherActor :type Actor%20Object%20Reference)))

(event EventTick
  (params (DeltaSeconds :type Float%20%28single-precision%29)))

(event EventEnemyAttackPlayer
  (Abilities|TryActivateAbilitiesbyTag (Variables|Default|GetASC) (GameplayTags|MakeLiteralGameplayTagContainer "(GameplayTags=((TagName=\"Attack.EnemyAttack\")))") true))

(fn ConstructionScript)